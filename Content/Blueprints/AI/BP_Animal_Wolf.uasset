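; Wolf animal Blueprint, a child class that animates its static mesh procedurally by changing its relative height.
; While velocity is non-zero, Tick keeps a looping timer for the movement bob, which AnimateMovement eases between two heights using FlipFlop.
; Jumping extends the parent function, playing a timeline that lifts the mesh, reverses it back down, then ends the gameplay behavior.
; When stationary and not jumping, the mesh returns to its starting height.
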(event Custom|Reverse
  (bind _staticmesh (Variables|Default|GetStaticMesh))
  (bind _defaultz (Variables|Default|GetDefaultZ))
  (bind _relativelocation (Variables|/Script/Engine.SceneComponent|GetRelativeLocation _staticmesh))
  (bind _alpha (Timeline|PlayJumping ReverseFromEnd)
    (:Update
      (Transformation|SetRelativeLocation (Variables|Default|GetStaticMesh) (Math|Vector|MakeVector (.x _relativelocation) (.y _relativelocation) (Math|Float|Lerp _defaultz (+ _defaultz 15.0) _alpha)) false false))
    (:Finished
      (if (!= (.z (Variables|/Script/Engine.SceneComponent|GetRelativeLocation (Variables|Default|GetStaticMesh))) (Variables|Default|GetDefaultZ))
        (CallFunction|Reverse)
        (else
          (Variables|Default|SetIsJumpPlaying false)
          (GameplayBehavior|EndBehavior (Variables|Default|GetGameplay%20Behavior) self))))))

(event EventBeginPlay
  (Variables|Default|SetDefaultZ (.z (Variables|/Script/Engine.SceneComponent|GetRelativeLocation (Variables|Default|GetStaticMesh)))))

(event Collision|EventActorBeginOverlap
  (params (OtherActor :type Actor%20Object%20Reference)))

(event EventTick
  (params (DeltaSeconds :type Float%20%28single-precision%29))
  (bind _staticmesh (Variables|Default|GetStaticMesh))
  (bind _relativelocation (Variables|/Script/Engine.SceneComponent|GetRelativeLocation _staticmesh))
  (if (> (Math|Vector|VectorLength (Variables|/Script/Engine.MovementComponent|GetVelocity (Variables|Character|GetCharacterMovement))) 0.0)
    (if (not (Utilities|Time|IsValidTimerHandle (Variables|Default|GetTimer)))
      (bind _returnvalue (Utilities|Time|SetTimerbyEvent (EventDispatchers|CreateEvent :!event AnimateMovement) (Utilities|Time|GetWorldDeltaSeconds) true))
      (Variables|Default|SetTimer _returnvalue))
    (else
      (Utilities|Time|ClearandInvalidateTimerbyHandle (Variables|Default|GetTimer))
      (if (not (Variables|Default|GetIsJumpPlaying))
        (Transformation|SetRelativeLocation (Variables|Default|GetStaticMesh) (Math|Vector|MakeVector (.x _relativelocation) (.y _relativelocation) (Variables|Default|GetDefaultZ)) false false)))))

(fn ConstructionScript
  (|CallParentFunction))

(fn Jumping
  (params (GameplayBehavior :type Gameplay%20Behavior%20Object%20Reference))
  (|CallParentFunction GameplayBehavior)
  (Variables|Default|SetIsJumpPlaying true)
  (Components|Timeline|PlayfromStart (Variables|Default|GetPlayJumping)))

(fn AnimateMovement
  (bind _staticmesh (Variables|Default|GetStaticMesh))
  (bind _defaultz (Variables|Default|GetDefaultZ))
  (bind _relativelocation (Variables|/Script/Engine.SceneComponent|GetRelativeLocation _staticmesh))
  (Transformation|SetRelativeLocation (Variables|Default|GetStaticMesh) (Math|Vector|MakeVector (.x _relativelocation) (.y _relativelocation) (Math|Interpolation|Ease "Linear" 0.2 (.z (Variables|/Script/Engine.SceneComponent|GetRelativeLocation (Variables|Default|GetStaticMesh))) (Math|Float|SelectFloat (+ _defaultz 5.0) _defaultz (Variables|Default|GetFlipFlop)))) false false)
  (if (Math|Float|NearlyEqual(Float) (.z (Variables|/Script/Engine.SceneComponent|GetRelativeLocation (Variables|Default|GetStaticMesh))) (Math|Float|SelectFloat (+ _defaultz 5.0) _defaultz (Variables|Default|GetFlipFlop)) 0.1)
    (Variables|Default|SetFlipFlop (not (Variables|Default|GetFlipFlop)))))